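; Minesweeper-style board actor that builds a grid of BP_Tile actors on BeginPlay and answers neighbor mine queries.
; Tiles spawn 100 units apart on the YZ plane, each randomly mined by MineChance, and fill a flattened Squares array.
; A second pass hands each tile its board reference and coordinates.
; Bounds-checked GetTile lets GetSurroundingMineCount sum mines over a 3x3 block, center included.
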(event EventBeginPlay
  (CallFunction|CreateBoard))

(fn ConstructionScript)

(fn CreateBoard
  (bind _x (LocalVariables|Getx))
  (bind _y (LocalVariables|Gety))
  (Utilities|FlowControl|Sequence
    (:then_0
      (Utilities|Array|Resize (Variables|Default|Getsquares) (* (Variables|Default|Getboard%20width) (Variables|Default|Getboard%20height))))
    (:then_1
      (|IterateOverBoard)
      (bind _returnvalue (Game|SpawnActorfromClass (Variables|Default|Getto%20spawn) (|maketransformforposition) false))
      (bind _asbp_tile_c (Utilities|Casting|CastToBP_Tile _returnvalue))
      (CallFunction|SetTile (LocalVariables|Getx) (LocalVariables|Gety) _asbp_tile_c)
      (if (<= (Math|Random|RandomFloat) (Variables|Default|Getmine%20chance))
        (Default|SetasMine _asbp_tile_c)))
    (:then_2
      (|iterateoverboardagain)
      (bind _tile (CallFunction|GetTile _x _y))
      (Default|SetBoard _tile self _x _y))))

(fn SetTile
  (params (x :type Integer) (y :type Integer) (tile :type BP%20Tile%20Object%20Reference))
  (Utilities|Array|SetArrayElem (Variables|Default|Getsquares) (+ x (* y (Variables|Default|Getboard%20width))) tile))

(fn GetTile
  (params (x :type Integer) (y :type Integer))
  (LocalVariables|Settx x)
  (LocalVariables|Setty y)
  (Utilities|FlowControl|Sequence
    (:then_0
      (LocalVariables|Setvalid%20position (Math|Boolean|ORBoolean (< (LocalVariables|Gettx) 0) (< (LocalVariables|Getty) 0) (>= (LocalVariables|Gettx) (Variables|Default|Getboard%20width)) (>= (LocalVariables|Getty) (Variables|Default|Getboard%20height)))))
    (:then_1
      (if (LocalVariables|Getvalid%20position)
        _
        (else
          (LocalVariables|Setto%20return (Utilities|Array|Get(acopy) (Variables|Default|Getsquares) (+ (LocalVariables|Gettx) (* (LocalVariables|Getty) (Variables|Default|Getboard%20width)))))))
      (return (LocalVariables|Getto%20return) (not (LocalVariables|Getvalid%20position))))))

(fn GetSurroundingMineCount
  (params (x :type Integer) (y :type Integer))
  (Utilities|FlowControl|Sequence
    (:then_0
      (LocalVariables|Setminecount 0)
      (LocalVariables|Setmin%20x (- x 1))
      (LocalVariables|Setmax%20x (+ x 1))
      (LocalVariables|Setmin%20y (- y 1))
      (LocalVariables|Setmax%20y (+ y 1)))
    (:then_1
      (for _index (range (LocalVariables|Getmin%20x) (LocalVariables|Getmax%20x))
        (for _index_2 (range (LocalVariables|Getmin%20y) (LocalVariables|Getmax%20y))
          (bind (_tile _is_valid) (CallFunction|GetTile _index _index_2))
          (if _is_valid
            (LocalVariables|Settile _tile)
            (LocalVariables|Setminecount (+ (Math|Conversions|ToInteger(Boolean) (Variables|/Game/Blueprints/BP_Tile.BP_Tile_C|Getis%20mine (LocalVariables|Gettile))) (LocalVariables|Getminecount)))))))
    (:then_2
      (return (LocalVariables|Getminecount)))))