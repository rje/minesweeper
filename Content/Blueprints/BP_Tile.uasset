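; BP_Tile is a single board tile for a touch-driven Minesweeper-style game, showing either a mine marker or its surrounding mine count.
; Construction creates a dynamic material and caches its base color for a timeline-driven flash that fades from white.
; SetAsMine flags the tile and shows an asterisk, while SetBoard stores coordinates and displays the board's neighbor count on non-mines.
; Touching the tile sets its text to "T" and plays the flash.
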(event EventActorOnInputTouchBegin
  (params (FingerIndex :type ETouchIndex%20Enum :default "Touch1"))
  (Rendering|Components|TextRender|SetText (Variables|Default|GetTextRender1) "T")
  (|FlashTile))

(fn ConstructionScript
  (bind _returnvalue (Rendering|Material|CreateDynamicMaterialInstance "/Game/Materials/Mat_Tile.Mat_Tile" :!class /Script/Engine.KismetMaterialLibrary))
  (Variables|Default|Setbox%20material _returnvalue)
  (Rendering|Material|SetMaterial (Variables|Default|GetStaticMesh1) 0 (Variables|Default|Getbox%20material))
  (bind _returnvalue_2 (Rendering|Material|GetVectorParameterValue (Variables|Default|Getbox%20material) "Color" :!class /Script/Engine.MaterialInstanceDynamic))
  (Variables|Default|Setbase%20color _returnvalue_2))

(fn FlashTile
  (params (perc :type Float%20%28single-precision%29))
  (Rendering|Material|SetVectorParameterValue (Variables|Default|Getbox%20material) "Color" (Math|Color|Lerp(LinearColor) "(R=1.000000,G=1.000000,B=1.000000,A=1.000000)" (Variables|Default|Getbase%20color) (- 1.0 perc)) :!class /Script/Engine.MaterialInstanceDynamic))

(fn SetasMine
  (Variables|Default|Setis%20mine true)
  (Rendering|Components|TextRender|SetText (Variables|Default|GetTextRender1) "*"))

(fn SetBoard
  (params (board :type BP%20Board%20Object%20Reference) (x :type Integer) (y :type Integer))
  (Variables|Default|Setboard board)
  (Variables|Default|Setx x)
  (Variables|Default|Sety y)
  (bind _count (Default|GetSurroundingMineCount (Variables|Default|Getboard) (Variables|Default|Getx) (Variables|Default|Gety)))
  (Variables|Default|Setsurrounding%20mine%20count _count)
  (if (not (Variables|Default|Getis%20mine))
    (Rendering|Components|TextRender|SetText (Variables|Default|GetTextRender1) (Utilities|String|ToString(Integer) _count))))